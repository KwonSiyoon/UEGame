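; BP_Weapon is a pickup melee weapon that a player collects and uses to deal damage.
; Overlapping its collect collision hands it to BP_Player via OnWeaponCollect, records that player as owner and disables further pickup.
; An attack collision starts disabled and is enabled as query-only between AttackCheckBegin and AttackCheckEnd events.
; Overlaps on it apply damage credited to the owner's controller, with the weapon as causer.
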(event `self.ReceiveBeginPlay`
  (`PrimitiveComponent.SetCollisionEnabled` (`self.AttackCollision`) "NoCollision"))

(event `self.CollectCollision.OnComponentBeginOverlap`
  (params (OverlappedComponent :type "PrimitiveComponent Object Reference") (OtherActor :type "Actor Object Reference") (OtherComp :type "PrimitiveComponent Object Reference") (OtherBodyIndex :type Integer) (bFromSweep :type Boolean) (SweepResult :type "HitResult Structure (by ref)"))
  (bind _asbp_player (cast `/Game/Blueprints/BP_Player` OtherActor))
  (`/Game/Blueprints/BP_Player.OnWeaponCollect` _asbp_player self)
  (set `self.MyOwner` _asbp_player)
  (`PrimitiveComponent.SetCollisionEnabled` (`self.CollectCollision`) "NoCollision"))

(event `AttackCheckBegin`
  (`PrimitiveComponent.SetCollisionEnabled` (`self.AttackCollision`) "QueryOnly"))

(event `AttackCheckEnd`
  (`PrimitiveComponent.SetCollisionEnabled` (`self.AttackCollision`) "NoCollision"))

(event `self.AttackCollision.OnComponentBeginOverlap`
  (params (OverlappedComponent :type "PrimitiveComponent Object Reference") (OtherActor :type "Actor Object Reference") (OtherComp :type "PrimitiveComponent Object Reference") (OtherBodyIndex :type Integer) (bFromSweep :type Boolean) (SweepResult :type "HitResult Structure (by ref)"))
  (bind _myowner (`self.MyOwner`))
  (`/Engine/EditorBlueprintResources/StandardMacros.IsValid` _myowner
    (:`Is Valid`
      (`GameplayStatics.ApplyDamage` OtherActor (`self.Damage`) (`Pawn.GetController` _myowner) self))))

(fn `UserConstructionScript`)