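; BP_Monster is an enemy monster (fire golem material) that chases, attacks and takes damage from BP_Player.
; SetState mirrors the state into a Blackboard key, with BT_Golem calling back after hits, while PawnSensing starts the chase and leaving ChaseRange returns it to Idle.
; An attack collision, toggled by attack-check events, applies damage, and incoming damage goes to BPDamageReceiver.
; Timelines drive material parameters for hit flashes and a death dissolve before destroying the actor.
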(event `SetState`
  (params (NewState :type "/Game/Blueprints/E_Monster Enum" :default "NewEnumerator0"))
  ;[1 1 1] Set State
  (if (`|EnumInequality` (`self.State`) "NewEnumerator3")
    (if (`|EnumInequality` (`self.State`) NewState)
      (bind _output_get (set `self.State` NewState))
      (`BlackboardComponent.SetValueAsEnum` (`AIBlueprintHelperLibrary.GetBlackboard` (`AIBlueprintHelperLibrary.GetAIController` self)) (`self.StateKey`) _output_get))))

(event `self.ReceiveBeginPlay`
  (set `PawnSensingComponent.SightRadius` (`self.ChaseRange`) (`self.PawnSensing`))
  (`PrimitiveComponent.SetCollisionEnabled` (`self.AttackCollision`) "NoCollision")
  (add `/Game/Blueprints/BP_DamageReceiver.OnDead` (`self.BP_DamageReceiver`) (delegate `OnDead`))
  (bind _returnvalue (`PrimitiveComponent.CreateDynamicMaterialInstance` (`self.Mesh`) 0 "/Game/InfinityBladeAdversaries/Enemy/Enemy_Golem/Materials/CharM_Fire_Golem_Inst.CharM_Fire_Golem_Inst" "None"))
  (set `self.DynamicInstance` _returnvalue))

(event `OnDead`
  (bind _mesh (`self.Mesh`))
  (`PrimitiveComponent.SetCollisionEnabled` (`self.CapsuleComponent`) "NoCollision")
  (`self.SetState` "NewEnumerator3")
  (bind (_direction _dissolve _dissolvecolor) (`Timeline|DeadDissolve` :!via `PlayFromStart`)
    (:`Update`
      (`MeshComponent.SetScalarParameterValueOnMaterials` _mesh "Dissolve" _dissolve)
      (`MeshComponent.SetScalarParameterValueOnMaterials` _mesh "HitValue" (* _dissolve 100.0))
      (`MeshComponent.SetVectorParameterValueOnMaterials` _mesh "HitColor" (`KismetMathLibrary.Conv_LinearColorToVector` _dissolvecolor)))
    (:`Finished`
      (`self.K2_DestroyActor`))))

(event `self.PawnSensing.OnSeePawn`
  (params (Pawn :type "Pawn Object Reference"))
  ;[1 1 1] Pawn Sensing
  (if (`|EnumEquality` (`self.State`) "NewEnumerator0")
    (bind _asbp_player (cast `/Game/Blueprints/BP_Player` Pawn))
    (if (`|EnumInequality` (`/Game/Blueprints/BP_Player.State` _asbp_player) "NewEnumerator2")
      (`self.SetState` "NewEnumerator1")
      (bind _output_get (set `self.Instigator` Pawn))
      (`BlackboardComponent.SetValueAsObject` (`AIBlueprintHelperLibrary.GetBlackboard` null) (`self.TargetKey`) _output_get))))

(event `self.ReceiveTick`
  (params (DeltaSeconds :type "Float (single-precision)"))
  (switch `/Game/Blueprints/E_Monster` (`self.State`)
    (:`NewEnumerator1`
      (`self.OnChase`))))

(event `OnAttackCheckBegin`
  ;[1 1 1] Attack Check
  (`PrimitiveComponent.SetCollisionEnabled` (`self.AttackCollision`) "QueryOnly"))

(event `OnAttackCheckEnd`
  ;[1 1 1] Attack Check
  (`PrimitiveComponent.SetCollisionEnabled` (`self.AttackCollision`) "NoCollision"))

(event `self.AttackCollision.OnComponentBeginOverlap`
  (params (OverlappedComponent :type "PrimitiveComponent Object Reference") (OtherActor :type "Actor Object Reference") (OtherComp :type "PrimitiveComponent Object Reference") (OtherBodyIndex :type Integer) (bFromSweep :type Boolean) (SweepResult :type "HitResult Structure (by ref)"))
  ;[1 1 1] Attack
  (bind _asbp_player (cast `/Game/Blueprints/BP_Player` OtherActor))
  (`GameplayStatics.ApplyDamage` _asbp_player (`self.Damage`) (`self.GetController`) self))

(event `self.ReceiveAnyDamage`
  (params (Damage :type "Float (single-precision)") (DamageType :type "DamageType Object Reference") (InstigatedBy :type "Controller Object Reference") (DamageCauser :type "Actor Object Reference"))
  ;[1 1 1] Damaged
  (bind _output_get (set `self.Instigator` (`Controller.K2_GetPawn` InstigatedBy)))
  (`/Engine/EditorBlueprintResources/StandardMacros.IsValid` _output_get
    (:`Is Valid`
      (bind _asbp_player (cast `/Game/Blueprints/BP_Player` _output_get))
      (`BlackboardComponent.SetValueAsObject` (`AIBlueprintHelperLibrary.GetBlackboard` null) (`self.TargetKey`) _asbp_player)
      (`self.SetState` "NewEnumerator4")
      (`/Game/Blueprints/BP_DamageReceiver.ReceiveDamage` (`self.BP_DamageReceiver`) Damage)
      (bind (_direction _hitvalue) (`Timeline|HitEffect` :!via `PlayFromStart`)
        (:`Update`
          (`MeshComponent.SetScalarParameterValueOnMaterials` (`self.Mesh`) "HitValue" _hitvalue))))))

(event `OnChase`
  (bind _instigator (`self.Instigator`))
  ;[1 1 1] 추적 범위 벗어나면 Idle로 변경
  (`/Engine/EditorBlueprintResources/StandardMacros.IsValid` _instigator
    (:`Is Valid`
      (if (> (`KismetMathLibrary.Vector_Distance` (`self.K2_GetActorLocation` _instigator) (`self.K2_GetActorLocation`)) (`self.ChaseRange`))
        (set `self.Instigator` null)
        (`self.SetState` "NewEnumerator0")))))

(event `OnDamaged`
  (bind _instigator (`self.Instigator`))
  ;[1 1 1] Damage 받은 후 State 판단 (BT_Golem에서 호출해줌.)
  (`/Engine/EditorBlueprintResources/StandardMacros.IsValid` _instigator
    (:`Is Valid`
      (if (> (`KismetMathLibrary.Vector_Distance` (`self.K2_GetActorLocation` _instigator) (`self.K2_GetActorLocation`)) (`self.ChaseRange`))
        (set `self.Instigator` null)
        (`self.SetState` "NewEnumerator0")
        (else
          (`self.SetState` "NewEnumerator1"))))))

(fn `ChangeState`
  (params (NewState :type "/Game/Blueprints/E_Monster Enum" :default "NewEnumerator0"))
  (if (`|EnumInequality` (`self.State`) "NewEnumerator3")
    (set `self.State` NewState)))

(fn `UserConstructionScript`)