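; BP_Bear is an AI-controlled bear character with sight sensing and a melee attack collision.
; BeginPlay sets sight radius from ChaseRange, creates a dynamic stone material and binds OnDead to the damage receiver.
; SetState mirrors state changes to the Blackboard, locking once the fourth enum value is reached.
; Attack check events toggle the hit collision; OnDead and OnDamaged are empty.
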(event `self.ReceiveBeginPlay`
  (`PrimitiveComponent.SetCollisionEnabled` (`self.AttackCollision`) "NoCollision")
  (set `PawnSensingComponent.SightRadius` (`self.ChaseRange`) (`self.PawnSensing`))
  (bind _returnvalue (`PrimitiveComponent.CreateDynamicMaterialInstance` (`self.Mesh`) 0 "/Game/InfinityBladeAdversaries/Enemy/Enemy_Bear/Materials/M_Bear_Stone_Inst.M_Bear_Stone_Inst" "None"))
  (set `self.DynamicInstance` _returnvalue)
  (add `/Game/Blueprints/BP_DamageReceiver.OnDead` (`self.BP_DamageReceiver`) (delegate `OnDead`)))

(event `OnDead`)

(event `SetState`
  (params (NewState :type "/Game/Blueprints/E_Monster Enum" :default "NewEnumerator0"))
  (bind _state (`self.State`))
  (if (`|EnumInequality` _state NewState)
    (if (`|EnumInequality` _state "NewEnumerator3")
      (bind _output_get (set `self.State` NewState))
      (`BlackboardComponent.SetValueAsEnum` (`AIBlueprintHelperLibrary.GetBlackboard` (`AIBlueprintHelperLibrary.GetAIController` self)) (`self.StateKey`) _output_get))))

(event `OnAttackCheckBegin`
  (`PrimitiveComponent.SetCollisionEnabled` (`self.AttackCollision`) "QueryOnly"))

(event `OnAttackCheckEnd`
  (`PrimitiveComponent.SetCollisionEnabled` (`self.AttackCollision`) "NoCollision"))

(event `OnDamaged`)

(fn `UserConstructionScript`)