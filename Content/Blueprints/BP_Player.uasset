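; Player character Blueprint handling Enhanced Input movement, look, jump, timeline dash, melee combat and death.
; A state enum gates actions; attacking needs a collected, socket-attached weapon and queues a four-section montage combo through NextCombo.
; Attack-check events forward to the weapon, while radial attack and BeginPlay sequence are signalled through separate calls.
; BPDamageReceiver takes non-self damage alongside camera shake; its death event disables capsule collision and removes input mapping.
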(event `self.ReceiveBeginPlay`
  (bind _returnvalue (`GameplayStatics.GetPlayerController` 0))
  (`/Engine/EditorBlueprintResources/StandardMacros.IsValid` _returnvalue
    (:`Is Valid`
      (`EnhancedInputSubsystemInterface.AddMappingContext` (pcsubsystem `EnhancedInputLocalPlayerSubsystem` _returnvalue) "/Game/Blueprints/IMC_InputManager.IMC_InputManager" 0 (struct))
      (add `/Game/Blueprints/BP_DamageReceiver.OnDead` (`self.BP_DamageReceiver`) (delegate `OnDead`))
      (`self.PlaySeqeunce`))))

(event `OnDead`
  (`PrimitiveComponent.SetCollisionEnabled` (`self.CapsuleComponent`) "NoCollision")
  (set `self.State` "NewEnumerator2")
  (bind `_as플레이어_컨트롤러` (cast `PlayerController` (`self.GetController` self)))
  (`EnhancedInputSubsystemInterface.RemoveMappingContext` (pcsubsystem `EnhancedInputLocalPlayerSubsystem` `_as플레이어_컨트롤러`) "/Game/Blueprints/IMC_InputManager.IMC_InputManager" (struct)))

(event `EnhancedInput|/Game/ThirdPerson/Input/Actions/IA_Move`
  (params (ActionValue :type "Vector2D Structure") (ElapsedSeconds :type "Float (double-precision)") (TriggeredSeconds :type "Float (double-precision)") (InputAction :type "InputAction Object Reference" :default "/Game/ThirdPerson/Input/Actions/IA_Move.IA_Move"))
  (bind (_returnvalue_roll _returnvalue_pitch _returnvalue_yaw) (`KismetMathLibrary.BreakRotator` (`self.GetControlRotation`)))
  ;[1 1 1] 이동, 회전, 점프
  (:`Triggered`
    (if (`|EnumEquality` (`self.State`) "NewEnumerator0")
      (`self.AddMovementInput` (+ (* ActionValue_X (`KismetMathLibrary.GetRightVector` (`KismetMathLibrary.MakeRotator` 0.0 0.0 _returnvalue_yaw))) (* ActionValue_Y (`KismetMathLibrary.GetForwardVector` (`KismetMathLibrary.MakeRotator` 0.0 0.0 _returnvalue_yaw))))))))

(event `EnhancedInput|/Game/Blueprints/IA_Attack`
  (params (ActionValue :type Boolean) (ElapsedSeconds :type "Float (double-precision)") (TriggeredSeconds :type "Float (double-precision)") (InputAction :type "InputAction Object Reference" :default "/Game/Blueprints/IA_Attack.IA_Attack"))
  ;[1 1 1] AttackSystem
  (:`Triggered`
    (if (and (not (`NavMovementComponent.IsFalling` (`self.CharacterMovement`))) (`self.bHasWeapon`))
      (if (`|EnumInequality` (`self.State`) "NewEnumerator1")
        (set `self.State` "NewEnumerator1")
        (`self.PlayAnimMontage` "/Game/Blueprints/AM_Warrior.AM_Warrior" 1.0 "Attack1")
        (else
          (switch `name` (`AnimInstance.Montage_GetCurrentSection` (`SkeletalMeshComponent.GetAnimInstance` (`self.Mesh`)) null)
            (:`Attack1`
              (set `self.NextCombo` "Attack2"))
            (:`Attack2`
              (set `self.NextCombo` "Attack3"))
            (:`Attack3`
              (set `self.NextCombo` "Attack4"))
            (:`Attack4`
              (set `self.NextCombo` "Attack1"))))))))

(event `EnhancedInput|/Game/ThirdPerson/Input/Actions/IA_Look`
  (params (ActionValue :type "Vector2D Structure") (ElapsedSeconds :type "Float (double-precision)") (TriggeredSeconds :type "Float (double-precision)") (InputAction :type "InputAction Object Reference" :default "/Game/ThirdPerson/Input/Actions/IA_Look.IA_Look"))
  ;[1 1 1] 이동, 회전, 점프
  (:`Triggered`
    (if (`|EnumInequality` (`self.State`) "NewEnumerator3")
      (`self.AddControllerPitchInput` ActionValue_Y)
      (`self.AddControllerYawInput` ActionValue_X))))

(event `EnhancedInput|/Game/ThirdPerson/Input/Actions/IA_Jump`
  (params (ActionValue :type Boolean) (ElapsedSeconds :type "Float (double-precision)") (TriggeredSeconds :type "Float (double-precision)") (InputAction :type "InputAction Object Reference" :default "/Game/ThirdPerson/Input/Actions/IA_Jump.IA_Jump"))
  ;[1 1 1] 이동, 회전, 점프
  (:`Triggered`
    (if (`|EnumEquality` (`self.State`) "NewEnumerator0")
      (`self.Jump`))))

(event `OnAttack`)

(event `self.ReceiveAnyDamage`
  (params (Damage :type "Float (single-precision)") (DamageType :type "DamageType Object Reference") (InstigatedBy :type "Controller Object Reference") (DamageCauser :type "Actor Object Reference"))
  ;[1 1 1] Damaged
  (if (!= (`Controller.K2_GetPawn` InstigatedBy) self)
    (`/Game/Blueprints/BP_DamageReceiver.ReceiveDamage` (`self.BP_DamageReceiver`) Damage)
    (`PlayerCameraManager.StartCameraShake` :`self` (`GameplayStatics.GetPlayerCameraManager` 0) :`ShakeClass` "/Game/Blueprints/BP_CameraShake.BP_CameraShake_C")))

(event `OnWeaponCollect`
  (params (WeaponActor :type "Actor Object Reference"))
  ;[1 1 1] 무기습득
  (`self.SetOwner` WeaponActor self)
  (bind _returnvalue (`self.K2_AttachToComponent` WeaponActor (`self.Mesh`) "WeaponPosition" "SnapToTarget" "KeepRelative" "KeepRelative" true))
  (set `self.bHasWeapon` _returnvalue)
  (bind _asbp_weapon (cast `/Game/Blueprints/BP_Weapon` WeaponActor))
  (set `self.MyWeapon` _asbp_weapon))

(event `EnhancedInput|/Game/Blueprints/IA_Dash`
  (params (ActionValue :type Boolean) (ElapsedSeconds :type "Float (double-precision)") (TriggeredSeconds :type "Float (double-precision)") (InputAction :type "InputAction Object Reference" :default "/Game/Blueprints/IA_Dash.IA_Dash"))
  (bind (_returnvalue_roll _returnvalue_pitch _returnvalue_yaw) (`KismetMathLibrary.BreakRotator` (`self.GetControlRotation`)))
  (bind (_returnvalue_x _returnvalue_y) (`KismetMathLibrary.BreakVector2D` (`|GetInputActionValue`)))
  ;[1 1 1] Dash
  (:`Triggered`
    (bind _output_get (set `self.DashDirection` (+ (* _returnvalue_x (`KismetMathLibrary.GetRightVector` (`KismetMathLibrary.MakeRotator` 0.0 0.0 _returnvalue_yaw))) (* _returnvalue_y (`KismetMathLibrary.GetForwardVector` (`KismetMathLibrary.MakeRotator` 0.0 0.0 _returnvalue_yaw))))))
    (set `self.DashStartLocation` (`self.K2_GetActorLocation`))
    (bind (_direction _lerp) (`Timeline|DashTimeLine` :!via `PlayFromStart`)
      (:`Update`
        (`self.K2_SetActorLocation` (+ (`self.DashStartLocation`) (* (* _lerp (`self.DashDistance`)) _output_get)))))))

(event `AttackCheckBegin`
  (bind _myweapon (`self.MyWeapon`))
  (`/Engine/EditorBlueprintResources/StandardMacros.IsValid` _myweapon
    (:`Is Valid`
      (`/Game/Blueprints/BP_Weapon.AttackCheckBegin` _myweapon))))

(event `AttackCheckEnd`
  (bind _myweapon (`self.MyWeapon`))
  (`/Engine/EditorBlueprintResources/StandardMacros.IsValid` _myweapon
    (:`Is Valid`
      (`/Game/Blueprints/BP_Weapon.AttackCheckEnd` _myweapon))))

(event `OnRadialAttack`
  (`self.RadialAttack`))

(fn `Turn to Target`
  (bind (_returnvalue_roll _returnvalue_pitch _returnvalue_yaw) (`KismetMathLibrary.BreakRotator` (`self.GetControlRotation`)))
  (`self.K2_SetActorRotation` (`KismetMathLibrary.MakeRotFromX` (`KismetMathLibrary.GetForwardVector` (`KismetMathLibrary.MakeRotator` 0.0 0.0 _returnvalue_yaw)))))

(fn `UserConstructionScript`)